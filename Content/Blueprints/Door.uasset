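; Door actor that raises its mesh vertically when activated by a switch and lowers it again on deactivation.
; BeginPlay stores the mesh's starting world location, and a timeline elevation track is added to its Z as the timeline plays.
; Deactivation reverses the timeline unless the StayOpen flag is set, which keeps the door open.
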(event `self.ReceiveBeginPlay`
  (set `self.InitialDoorLocation` (`SceneComponent.K2_GetComponentLocation` (`self.DoorMesh`))))

(event `/Game/Blueprints/SwitchInterface.Activate Switch`
  (bind (_direction _doorelevation) (`Timeline|DoorTimeline` :!label _label)
    (:`Update`
      (`SceneComponent.K2_SetWorldLocation` (`self.DoorMesh`) (`KismetMathLibrary.MakeVector` (.x (`self.InitialDoorLocation`)) (.y (`self.InitialDoorLocation`)) (+ (.z (`self.InitialDoorLocation`)) _doorelevation)) false false))))

(event `/Game/Blueprints/SwitchInterface.Deactivate Switch`
  (if (not (`self.StayOpen`))
    (goto _label :!via `Reverse`)))

(fn `UserConstructionScript`)