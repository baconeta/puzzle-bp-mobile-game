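; Player controller for a touch-driven puzzle game where the player selects and moves PuzzleCharacters viewed through per-character camera volumes.
; Tick turns finger drags into interpolated rotation of the focused volume's camera.
; Short taps select, switch or deselect characters, possessing and blending views on selection, or send the selected one to the tapped point via SimpleMoveToLocation.
; Switching restores camera transforms and spline following; the mouse-move gate's Enter is unwired.
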(event `self.ReceiveBeginPlay`
  (set `self.bShowMouseCursor` true)
  (bind _aspuzzle_character (cast `/Game/Blueprints/Character/PuzzleCharacter` (`GameplayStatics.GetPlayerPawn` 0)))
  (bind _output_get (set `self.FocusedCameraVolume` (`/Game/Blueprints/Character/PuzzleCharacter.CurrentCameraVolume` _aspuzzle_character)))
  (`self.SetViewTargetWithBlend` _output_get))

(event `self.ReceiveTick`
  (params (DeltaSeconds :type "Float (single-precision)"))
  (bind (_locationx _locationy) (`self.GetInputTouchState` "Touch1"))
  (bind (_camera _returnvalue) (`self.AddToCameraRotation`))
  (bind (_x _y) (`KismetMathLibrary.BreakVector2D` (`self.PreviousTouchLocation`)))
  (if (`self.FingerPressed`)
    (set `self.Delta Seconds` DeltaSeconds)
    (set `self.CurrentTouchLocation` (`KismetMathLibrary.MakeVector2D` _locationx _locationy))
    (if (and (== _x -1.0) (== _y -1.0))
      (set `self.PreviousTouchLocation` (`self.CurrentTouchLocation`))
      (else
        (set `self.DeltaTouchLocation` (- (`self.PreviousTouchLocation`) (`self.CurrentTouchLocation`)))
        (`SceneComponent.K2_SetWorldRotation` _camera _returnvalue false false)
        (set `self.PreviousTouchLocation` (`self.CurrentTouchLocation`))))))

(event `InputTouch`
  (params (Location :type "Vector Structure") (FingerIndex :type "ETouchIndex Enum"))
  (bind _returnvalue (`|EnumEquality` FingerIndex "Touch1"))
  ;[1 1 1] Touch movement and player selections
  (:`Pressed`
    (if _returnvalue
      (`self.TouchPressed`)))
  (:`Released`
    (if _returnvalue
      (`self.Touch Released`))))

(event `InputAction|SetDestination`
  (params (Key :type "Key Structure"))
  ;[1 1 1] Mouse input movement
  (:`Pressed`
    (`/Engine/EditorBlueprintResources/StandardMacros.Gate` true :!via `Open` :!label _label
      (:`Exit`
        (`self.Move to Hit Location` (`.Location` (`GameplayStatics.BreakHitResult` (`self.GetHitResultUnderCursorByChannel` "TraceTypeQuery1")))))))
  (:`Released`
    (goto _label :!via `Close`)))

(fn `AddToCameraRotation`
  (returns (Camera :type "CameraComponent Object Reference") (ReturnValue :type "Rotator Structure"))
  (bind _swipespeed (`self.SwipeSpeed`))
  (bind (_x _y) (`KismetMathLibrary.BreakVector2D` (`self.DeltaTouchLocation`)))
  (bind _camera (`/Game/Blueprints/CameraVolume.Camera` (`self.FocusedCameraVolume`)))
  (bind _returnvalue (`SceneComponent.K2_GetComponentRotation` _camera))
  (return _camera (`KismetMathLibrary.RInterpTo` _returnvalue (`KismetMathLibrary.MakeRotator` (.roll _returnvalue) (* (+ (.pitch _returnvalue) (* _y -1.0)) _swipespeed) (* (+ (.yaw _returnvalue) _x) _swipespeed)) (`self.Delta Seconds`) 3.0)))

(fn `Change Selected Character`
  (locals (PreviousCameraTransform :type "Transform Structure") (UsePreviousCameraTransform :type Boolean))
  (bind _selectedcharacter (`self.SelectedCharacter`))
  (bind _previouscameravolume (`self.PreviousCameraVolume`))
  (bind _focusedcameravolume (`self.FocusedCameraVolume`))
  (bind _currentcameravolume (`/Game/Blueprints/Character/PuzzleCharacter.CurrentCameraVolume` (`self.HitCharacter`)))
  (bind _currentcameravolume_2 (`/Game/Blueprints/Character/PuzzleCharacter.CurrentCameraVolume` _selectedcharacter))
  (bind _camera (`/Game/Blueprints/CameraVolume.Camera` _previouscameravolume))
  (if (== (`/Game/Blueprints/Character/PuzzleCharacter.CurrentCameraVolume` (`self.SelectedCharacter`)) _currentcameravolume)
    (set `local.PreviousCameraTransform` (`SceneComponent.K2_GetComponentToWorld` (`/Game/Blueprints/CameraVolume.Camera` _currentcameravolume)))
    (set `local.UsePreviousCameraTransform` true)
    (else
      (set `local.UsePreviousCameraTransform` false)))
  (set `self.PreviousCameraVolume` (`/Game/Blueprints/Character/PuzzleCharacter.CurrentCameraVolume` (`self.SelectedCharacter`)))
  ;[1 1 1] Unselect character
  (`/Game/Blueprints/Character/PuzzleCharacter.DisableSelectionWidget` (`self.SelectedCharacter`))
  (`self.UnPossess`)
  ;[1 1 1] Select the hit character
  (bind _output_get (set `self.SelectedCharacter` (`self.HitCharacter`)))
  (`/Game/Blueprints/Character/PuzzleCharacter.EnableSelectionWidget` _output_get)
  (`self.Possess` _selectedcharacter)
  (set `/Game/Blueprints/CameraVolume.Character` (`self.SelectedCharacter`) _currentcameravolume_2)
  (set `self.FocusedCameraVolume` _currentcameravolume_2)
  (`self.SetViewTargetWithBlend` _currentcameravolume_2 0.0 "VTBlend_EaseInOut")
  ;[1 1 1] Reset required cameras
  (`/Engine/EditorBlueprintResources/StandardMacros.IsValid` _previouscameravolume
    (:`Is Valid`
      (if (`local.UsePreviousCameraTransform`)
        (`SceneComponent.K2_SetWorldTransform` _camera (`local.PreviousCameraTransform`) false false)
        (else
          (`SceneComponent.K2_SetWorldTransform` _camera (`/Game/Blueprints/CameraVolume.InitialCameraTransform` _previouscameravolume) false false)))
      (set `self.PreviousCameraVolume` null)
      (if (`/Game/Blueprints/CameraVolume.TurnUseSplineBackOn` _focusedcameravolume)
        (set `/Game/Blueprints/CameraVolume.UseSpline` true _focusedcameravolume)))))

(fn `Move to Hit Location`
  (params (HitLocation :type "Vector Structure"))
  (if (>= (`KismetMathLibrary.VSize` (- HitLocation (`self.K2_GetActorLocation` (`GameplayStatics.GetPlayerPawn` 0)))) (`self.MinClickDistance`))
    (`AIBlueprintHelperLibrary.SimpleMoveToLocation` self HitLocation)))

(fn `Touch Released`
  (bind (_locationx _locationy) (`self.GetInputTouchState` "Touch1"))
  (bind _focusedcameravolume (`self.FocusedCameraVolume`))
  (bind _hitactor (`self.HitActor`))
  (bind _currentcameravolume (`/Game/Blueprints/Character/PuzzleCharacter.CurrentCameraVolume` (`self.SelectedCharacter`)))
  (set `self.FingerPressed` false)
  (set `self.PreviousTouchLocation` (-1.0 -1.0))
  (bind _output_get (set `self.FinalTouchLocation` (`KismetMathLibrary.MakeVector2D` _locationx _locationy)))
  (if (<= (`KismetMathLibrary.VSize2D` (- (`self.InitialTouchLocation`) _output_get)) (`self.MinDragThreshold`))
    (`/Engine/EditorBlueprintResources/StandardMacros.IsValid` _hitactor
      (:`Is Valid`
        (bind _aspuzzle_character (cast `/Game/Blueprints/Character/PuzzleCharacter` _hitactor)
          (:`then`
            (set `self.HitCharacter` _aspuzzle_character)
            ;[1 1 1] Already have char selected?
            (`/Engine/EditorBlueprintResources/StandardMacros.IsValid` (`self.SelectedCharacter`)
              (:`Is Valid`
                ;[1 1 1] Not clicking the same selected character
                (if (!= (`self.SelectedCharacter`) (`self.HitCharacter`))
                  (`self.Change Selected Character`)
                  (else
                    ;[1 1 1] Deselect SelectedCharacter
                    (`/Game/Blueprints/Character/PuzzleCharacter.DisableSelectionWidget` (`self.SelectedCharacter`))
                    (set `self.SelectedCharacter` null))))
              (:`Is Not Valid`
                ;[1 1 1] Select the hit character
                (bind _output_get_2 (set `self.SelectedCharacter` (`self.HitCharacter`)))
                (`/Game/Blueprints/Character/PuzzleCharacter.EnableSelectionWidget` _output_get_2)
                (set `self.FocusedCameraVolume` _currentcameravolume)
                (`self.Possess` (`self.HitCharacter`))
                (`self.SetViewTargetWithBlend` _currentcameravolume 0.0 "VTBlend_EaseInOut"))))
          (:`CastFailed`
            ;[1 1 1] Move selected character
            (`/Engine/EditorBlueprintResources/StandardMacros.IsValid` (`self.SelectedCharacter`)
              (:`Is Valid`
                (`self.Move to Hit Location` (`self.HitLocation`))
                (if (`/Game/Blueprints/CameraVolume.TurnUseSplineBackOn` _focusedcameravolume)
                  (set `/Game/Blueprints/CameraVolume.UseSpline` true _focusedcameravolume))))))))))

(fn `TouchPressed`
  (bind (_locationx _locationy) (`self.GetInputTouchState` "Touch1"))
  (bind (_bblockinghit _binitialoverlap _time _distance _location _impactpoint _normal _impactnormal _physmat _hitactor) (`GameplayStatics.BreakHitResult` (`self.GetHitResultUnderFingerByChannel` "Touch1" "TraceTypeQuery1")))
  (set `self.FingerPressed` true)
  (set `self.InitialTouchLocation` (`KismetMathLibrary.MakeVector2D` _locationx _locationy))
  (bind _output_get (set `self.HitActor` _hitactor))
  (set `self.HitLocation` _location)
  (bind _aspuzzle_character (cast `/Game/Blueprints/Character/PuzzleCharacter` _output_get))
  (set `/Game/Blueprints/CameraVolume.UseSpline` false (`/Game/Blueprints/Character/PuzzleCharacter.CurrentCameraVolume` _aspuzzle_character)))

(fn `UserConstructionScript`)