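; A switch-driven platform that rises like a door once enough switches are activated.
; Activate and deactivate events adjust a switch count; reaching the required number plays a sound and runs a timeline.
; The timeline offsets the platform's height from the position stored at BeginPlay.
; Dropping below the required count reverses the timeline unless the platform is set to stay open.
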(event `self.ReceiveBeginPlay`
  (set `self.InitialDoorLocation` (`SceneComponent.K2_GetComponentLocation` (`self.Platform`))))

(event `/Game/Blueprints/SwitchInterface.Activate Switch`
  (bind _switchesactivated (`self.SwitchesActivated`))
  (`/Engine/EditorBlueprintResources/StandardMacros.IncrementInt` _switchesactivated
    (:`  `
      (if (>= _switchesactivated (`self.SwitchesRequired`))
        (`GameplayStatics.PlaySound2D` (`self.DoorSound`) 1.0 1.0 0.0 null null)
        (bind (_direction _doorelevation) (`Timeline|DoorTimeline` :!label _label)
          (:`Update`
            (`SceneComponent.K2_SetWorldLocation` (`self.Platform`) (`KismetMathLibrary.MakeVector` (.x (`self.InitialDoorLocation`)) (.y (`self.InitialDoorLocation`)) (+ (.z (`self.InitialDoorLocation`)) _doorelevation)) false false)))))))

(event `/Game/Blueprints/SwitchInterface.Deactivate Switch`
  (`/Engine/EditorBlueprintResources/StandardMacros.DecrementInt` (`self.SwitchesActivated`)
    (:`  `
      (if (< (`self.SwitchesActivated`) (`self.SwitchesRequired`))
        (if (not (`self.StayOpen`))
          (goto _label :!via `Reverse`))))))

(fn `UserConstructionScript`)