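; PuzzleCharacter is a character Blueprint for a puzzle game that can jump and show a selection cursor.
; EnableSelectionWidget reveals the SelectionCursor widget component and plays its PlayerSelectIcon cursor animation on an endless loop.
; DisableSelectionWidget stops that animation and hides the cursor, and runs on BeginPlay so the character starts unselected.
; The Jump input action triggers the jump, while nothing in this Blueprint calls EnableSelectionWidget.
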(event `self.ReceiveBeginPlay`
  (`self.DisableSelectionWidget`))

(event `InputAction|Jump`
  (params (Key :type "Key Structure"))
  (:`Pressed`
    (`self.Jump`)))

(fn `DisableSelectionWidget`
  (bind _asplayer_select_icon (cast `/Game/HUD/PlayerSelectIcon` (`WidgetComponent.GetUserWidgetObject` (`self.SelectionCursor`))))
  (`UserWidget.StopAnimation` _asplayer_select_icon (`/Game/HUD/PlayerSelectIcon.CursorAnimation` _asplayer_select_icon))
  (`SceneComponent.SetVisibility` (`self.SelectionCursor`) false false))

(fn `EnableSelectionWidget`
  (bind _returnvalue (`WidgetComponent.GetUserWidgetObject` (`self.SelectionCursor`)))
  (bind _asplayer_select_icon (cast `/Game/HUD/PlayerSelectIcon` _returnvalue))
  (`UserWidget.PlayAnimation` _returnvalue (`/Game/HUD/PlayerSelectIcon.CursorAnimation` _asplayer_select_icon) 0.0 0 "Forward" 1.0 false)
  (`SceneComponent.SetVisibility` (`self.SelectionCursor`) true false))

(fn `UserConstructionScript`)