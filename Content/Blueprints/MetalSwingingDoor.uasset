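; A metal swinging door that opens once enough linked switches are active.
; Activate and deactivate switch events keep a count against a required threshold, playing a 2D sound as the door opens or closes.
; A timeline adds its track value to the root's initial yaw to swing the door.
; It reverses when the count drops below the threshold, unless StayOpen is set.
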(event `self.ReceiveBeginPlay`
  (set `self.InitialDoorLocation` (`SceneComponent.K2_GetComponentLocation` (`self.DoorMesh`)))
  (set `self.InitialDoorRotation` (`SceneComponent.K2_GetComponentRotation` (`self.DefaultSceneRoot`))))

(event `/Game/Blueprints/SwitchInterface.Activate Switch`
  (bind _switchesactivated (`self.SwitchesActivated`))
  (`/Engine/EditorBlueprintResources/StandardMacros.IncrementInt` _switchesactivated
    (:`  `
      (if (>= _switchesactivated (`self.SwitchesRequired`))
        (`GameplayStatics.PlaySound2D` (`self.DoorOpenSound`) 1.0 1.0 0.0 null null)
        (bind (_direction _doorelevation) (`Timeline|DoorTimeline` :!label _label)
          (:`Update`
            (`SceneComponent.K2_SetWorldRotation` (`self.DefaultSceneRoot`) (`KismetMathLibrary.MakeRotator` (.roll (`self.InitialDoorRotation`)) (.pitch (`self.InitialDoorRotation`)) (+ _doorelevation (.yaw (`self.InitialDoorRotation`)))) false false)))))))

(event `/Game/Blueprints/SwitchInterface.Deactivate Switch`
  (`/Engine/EditorBlueprintResources/StandardMacros.DecrementInt` (`self.SwitchesActivated`)
    (:`  `
      (if (< (`self.SwitchesActivated`) (`self.SwitchesRequired`))
        (if (not (`self.StayOpen`))
          (`GameplayStatics.PlaySound2D` (`self.DoorCloseSound`) 1.0 1.0 0.0 null null)
          (goto _label :!via `Reverse`))))))

(fn `UserConstructionScript`)